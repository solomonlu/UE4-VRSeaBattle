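; BP_FishingRod is a fishing rod actor that can be picked up and dropped, with a hook hanging from a cable.
; The construction script ties the Rod and Hook together with a physics constraint and sets the cable's end attachment to the actor itself.
; Each tick moves the cable end to the hook's position in actor space.
; Pickup disables rod physics and drop restores it, with no snapping to the interactor and a zero attach offset.
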(event `self.ReceiveTick`
  (params (DeltaSeconds :type "Float (single-precision)"))
  (set `CableComponent.EndLocation` (`KismetMathLibrary.InverseTransformLocation` (`self.GetTransform`) (`SceneComponent.K2_GetComponentLocation` (`self.Hook`))) (`self.Cable`)))

(event `/Game/ExampleContent/VR_World_Interaction/Blueprints/Interfaces/PickupableInterface.OnPickup`
  (`PrimitiveComponent.SetSimulatePhysics` (`self.Rod`) false))

(event `/Game/ExampleContent/VR_World_Interaction/Blueprints/Interfaces/PickupableInterface.OnDrop`
  (`PrimitiveComponent.SetSimulatePhysics` (`self.Rod`) true))

(fn `GetAttachLocation`
  (returns (Location :type "Vector Structure"))
  (return (0.0 0.0 0.0)))

(fn `ShouldSnapToInteractor`
  (returns (Snap :type Boolean))
  (return false))

(fn `UserConstructionScript`
  (`CableComponent.SetAttachEndTo` (`self.Cable`) self "None")
  (`PhysicsConstraintComponent.SetConstrainedComponents` (`self.PhysicsConstraint`) (`self.Rod`) "None" (`self.Hook`) "None"))