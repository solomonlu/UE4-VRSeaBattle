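; BP_Whale is a whale actor that swims forward and reacts to being harpooned.
; BeginPlay sets current health from MaxHealth, and Tick offsets the actor along its forward vector without sweeping.
; OnHarpoonInsert sets a flag that makes Tick drain health over time and move the whale ten times faster.
; Once health drops below zero it reverts to normal speed, with movement applied per frame, unscaled by delta time.
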(event `self.ReceiveBeginPlay`
  (set `self.CurHealth` (`KismetMathLibrary.Conv_IntToDouble` (`self.MaxHealth`))))

(event `self.ReceiveTick`
  (params (DeltaSeconds :type "Float (single-precision)"))
  (if (>= (`self.CurHealth`) 0.0)
    (if (`self.HarpoonInserted`)
      (set `self.CurHealth` (- (`self.CurHealth`) (* DeltaSeconds 10.0)))
      (`self.K2_AddActorWorldOffset` (* (`KismetMathLibrary.GetForwardVector` (`self.K2_GetActorRotation`)) (* (`self.MoveSpeed`) 10.0)))
      (else
        (`self.K2_AddActorWorldOffset` (* (`KismetMathLibrary.GetForwardVector` (`self.K2_GetActorRotation`)) (`self.MoveSpeed`)) :!label _label)))
    (else
      (goto _label))))

(event `/Game/Fish/Blueprints/Fishman/FishInterface.OnHarpoonInsert`
  (set `self.HarpoonInserted` true))

(fn `UserConstructionScript`)